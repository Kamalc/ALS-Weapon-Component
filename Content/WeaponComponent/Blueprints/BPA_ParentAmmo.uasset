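; Parent ammo pickup actor that offers ammo to overlapping actors and respawns after a delay.
; The construction script sets the particle template and builds a label from the ammo adding mode, or blanks it, for a name widget created at BeginPlay.
; On an authority-side overlap, it sends an AmmoPickupMessage with the ammo settings to the other actor.
; It then hides itself and its label and disables trigger collision until RespawnTime elapses.
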(event `self.ReceiveBeginPlay`
  (bind _returnvalue (`|CreateWidget` "/Game/WeaponComponent/UMG/W_ItemName.W_ItemName_C" null (`self.L_NameText`)))
  (`WidgetComponent.SetWidget` (`self.WidgetName`) _returnvalue))

(event `self.Trigger.OnComponentBeginOverlap`
  (params (OverlappedComponent :type "PrimitiveComponent Object Reference") (OtherActor :type "Actor Object Reference") (OtherComp :type "PrimitiveComponent Object Reference") (OtherBodyIndex :type Integer) (bFromSweep :type Boolean) (SweepResult :type "HitResult Structure (by ref)"))
  (`/Engine/EditorBlueprintResources/ActorMacros.Switch Has Authority`
    (:`Authority`
      (message `/Game/WeaponComponent/Blueprints/BPI_WpnComponent.AmmoPickup` OtherActor (`self.AmmoAddingType`) (`self.WeaponID`) (`self.AmountAmmo`) (`self.WeaponType`) (`self.ProjectileType`))
      (`self.ShowHideAmmo`))))

(event `ShowHideAmmo`
  (`self.SetActorHiddenInGame` self true)
  (`SceneComponent.SetVisibility` (`self.WidgetName`) false false)
  (`PrimitiveComponent.SetCollisionEnabled` (`self.Trigger`) "NoCollision")
  (`KismetSystemLibrary.Delay` (`self.RespawnTime`))
  (`self.SetActorHiddenInGame` self false)
  (`PrimitiveComponent.SetCollisionEnabled` (`self.Trigger`) "QueryOnly")
  (`SceneComponent.SetVisibility` (`self.WidgetName`) true false))

(fn `UserConstructionScript`
  (`ParticleSystemComponent.SetTemplate` (`self.ParticleSystem`) (`self.ParticleAmmo`))
  (if (`self.HideText`)
    (set `self.L_NameText` "")
    (else
      (set `self.L_NameText` (select `/Game/WeaponComponent/Blueprints/E_AddAmmoTypes` (`self.AmmoAddingType`) :`NewEnumerator0` "For CURRENT weapon (sample)" :`NewEnumerator1` "Large Ammo Pack     (for all weapons)     " :`NewEnumerator3` (`|FormatText` "For \"{WpnName}\" only" (`self.WeaponNameOrComment`)) :`NewEnumerator4` (`|FormatText` "Ammo for all {WpnType}s" (`KismetTextLibrary.Conv_StringToText` (`|GetEnumeratorNameAsString` (`self.WeaponType`)))) :`NewEnumerator2` (`KismetSystemLibrary.MakeLiteralText` (`self.WeaponNameOrComment`)))))))